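; BP_AbilityStatComponent is an actor component that tracks its owner's health between zero and a default maximum.
; On BeginPlay it binds to the owner's OnTakeAnyDamage and resets health, then subtracts incoming damage through AddHealth and prints the instigator and causer.
; AddHealth routes through SetHealth, which clamps the value and broadcasts OnChangeHealth with previous and current values.
; ResetHealth assigns the default directly, without broadcasting.
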(event `self.ReceiveBeginPlay`
  (add `Actor.OnTakeAnyDamage` (`self.GetOwner`) (delegate `커스텀이벤트_0`))
  (`self.ResetHealth`))

(event `커스텀이벤트_0`
  (params (DamagedActor :type "Actor Object Reference") (Damage :type "Float (double-precision)") (DamageType :type "DamageType Object Reference") (InstigatedBy :type "Controller Object Reference") (DamageCauser :type "Actor Object Reference"))
  (`self.AddHealth` (* Damage -1.0))
  (`KismetSystemLibrary.PrintString` (`KismetTextLibrary.Conv_TextToString` (`|FormatText` "Instigator{0}, Causer{1}" InstigatedBy DamageCauser))))

(fn `AddHealth`
  (params (Value :type "Float (double-precision)"))
  (`self.SetHealth` (+ (`self.Health`) Value)))

(fn `ResetHealth`
  (set `self.Health` (`self.DefaultHealth`)))

(fn `SetHealth`
  (params (Value :type "Float (double-precision)"))
  (locals (PrevHealth :type "Float (double-precision)"))
  (set `local.PrevHealth` (`self.Health`))
  (set `self.Health` (`KismetMathLibrary.FClamp` Value 0.0 (`self.DefaultHealth`)))
  (`self.OnChangeHealth` (`local.PrevHealth`) (`self.Health`)))